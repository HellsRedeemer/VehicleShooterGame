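; BP_BetterTank is a tank Blueprint with team colours, a spring arm and a widget that displays its network role.
; On BeginPlay it adds the actor's yaw to the spring arm's rotation and passes itself to the NetRole widget.
; SetTeamColours swaps the mesh's tracks material for red or blue by team.
; Pressing 3 calls Serverdam, which applies heavy damage to the tank itself, apparently as a debug shortcut.
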(event `self.ReceiveBeginPlay`
  (bind (_returnvalue_roll _returnvalue_pitch _returnvalue_yaw) (`KismetMathLibrary.BreakRotator` (`self.K2_GetActorRotation`)))
  (`SceneComponent.K2_AddRelativeRotation` (`self.SpringArm`) (`KismetMathLibrary.MakeRotator` 0.0 0.0 _returnvalue_yaw) false false)
  (bind _asnet_role (cast `/Game/Blueprints/NetRole` (`WidgetComponent.GetUserWidgetObject` (`self.Widget`))))
  (`/Game/Blueprints/NetRole.ShowNetRole` _asnet_role self))

(event `self.SetTeamColours`
  (bind _mesh (`self.Mesh`))
  (switch `ETeams` (`self.Team`)
    (:`ET_RedTeam`
      (`PrimitiveComponent.SetMaterial` _mesh 1 "/Game/VigilanteContent/Vehicles/West_Tank_M1A1Abrams/Materials/MI_TracksRed.MI_TracksRed"))
    (:`ET_BlueTeam`
      (`PrimitiveComponent.SetMaterial` _mesh 1 "/Game/VigilanteContent/Vehicles/West_Tank_M1A1Abrams/Materials/MI_TracksBlue.MI_TracksBlue"))))

(event `Key|Three`
  (params (Key :type "Key Structure"))
  (:`Pressed`
    (`self.serverdam`)))

(event `serverdam`
  (`GameplayStatics.ApplyDamage` self 3333.0))

(fn `UserConstructionScript`)