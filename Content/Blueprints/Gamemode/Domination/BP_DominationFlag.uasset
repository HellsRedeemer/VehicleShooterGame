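; Domination mode flag actor that displays a capture point's team and capture progress.
; UpdateFlag forwards capture percent, owner team and capturing team to ClientUpdateFlag, which feeds a WBP_TempCaptureWidget on its widget component.
; The mesh material changes only when percent is zero or below, following the capturing team, else the owner, else a neutral track material with the widget reset.
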(event `self.UpdateFlag`
  (params (CapurePercent :type "Float (single-precision)") (OwnerTeam :type "ETeams Enum" :default "ET_NoTeam") (CapturingTeam :type "ETeams Enum" :default "ET_NoTeam"))
  (`self.ClientUpdateFlag` CapurePercent OwnerTeam CapturingTeam))

(event `ClientUpdateFlag`
  (params (CapturePercent :type "Float (double-precision)") (OwnerTeam :type "ETeams Enum" :default "ET_NoTeam") (CapturingTeam :type "ETeams Enum" :default "ET_NoTeam"))
  (bind _staticmesh (`self.StaticMesh`))
  (bind _returnvalue (`WidgetComponent.GetWidget` (`self.Widget`)))
  (if (<= CapturePercent 0.0)
    (switch `ETeams` CapturingTeam
      (:`ET_NoTeam`
        (switch `ETeams` OwnerTeam
          (:`ET_NoTeam`
            (`PrimitiveComponent.SetMaterial` _staticmesh 0 "/Game/Track/M_Track.M_Track")
            (bind _aswbp_temp_capture_widget (cast `/Game/Blueprints/Gamemode/Domination/WBP_TempCaptureWidget` _returnvalue))
            (`/Game/Blueprints/Gamemode/Domination/WBP_TempCaptureWidget.UpdateCapPercent` _aswbp_temp_capture_widget 0.0 "ET_NoTeam"))
          (:`ET_RedTeam`
            (`PrimitiveComponent.SetMaterial` _staticmesh 0 "/Game/Track/MI_TrackEdge1.MI_TrackEdge1" :!label _label)
            (bind _aswbp_temp_capture_widget_2 (cast `/Game/Blueprints/Gamemode/Domination/WBP_TempCaptureWidget` _returnvalue :!label _label_2))
            (`/Game/Blueprints/Gamemode/Domination/WBP_TempCaptureWidget.UpdateCapPercent` _aswbp_temp_capture_widget_2 CapturePercent CapturingTeam))
          (:`ET_BlueTeam`
            (`PrimitiveComponent.SetMaterial` _staticmesh 0 "/Game/Track/MI_TrackEdge.MI_TrackEdge" :!label _label_3)
            (goto _label_2))))
      (:`ET_RedTeam`
        (goto _label))
      (:`ET_BlueTeam`
        (goto _label_3)))
    (else
      (goto _label_2))))

(fn `UserConstructionScript`)